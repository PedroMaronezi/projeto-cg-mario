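; BP_MainMenu is a menu actor that hosts a widget and moves the player's view to other linked menu actors.
; On BeginPlay it binds to the menu widget's transition event, via the WBP_MenuAbstractClass base, and turns its own collision off.
; When the widget sends a valid index into LinkedMenus, it disables its own collision, enables the target menu's, and blends the view target to that menu with ease-in-out.
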(event `self.ReceiveBeginPlay`
  (bind _aswbp_menu_abstract_class (cast `/Game/MainMenu/Widgets/WBP_MenuAbstractClass` (`WidgetComponent.GetUserWidgetObject` (`self.Widget`))))
  (add `/Game/MainMenu/Widgets/WBP_MenuAbstractClass.TransitionToLinkedMenu` _aswbp_menu_abstract_class (delegate `OnTransitionBetweenMenus`))
  (`self.SetActorEnableCollision` false))

(event `OnTransitionBetweenMenus`
  (params (MenuIndex :type Integer))
  (if (`KismetArrayLibrary.Array_IsValidIndex` (`self.LinkedMenus`) MenuIndex)
    (`self.TransitionTo` (`|GetArrayItem` (`self.LinkedMenus`) MenuIndex))))

(event `TransitionTo`
  (params (NewMenu :type "/Game/MainMenu/BP_MainMenu Object Reference"))
  (`self.SetActorEnableCollision` false)
  (`self.SetActorEnableCollision` NewMenu true)
  (`PlayerController.SetViewTargetWithBlend` (`GameplayStatics.GetPlayerController` 0) NewMenu (`self.BlendTime`) "VTBlend_EaseInOut" (`self.BlendExp`) false))

(fn `UserConstructionScript`)