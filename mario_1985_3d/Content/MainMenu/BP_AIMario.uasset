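; Main menu Mario character that runs on a loop, using AI MoveTo to reach a destination, then teleporting back to an origin and setting off again.
; Tick restarts the idle/walk animation whenever it has ended, flipbook-style by swapping static meshes through three walk frames on timed delays.
; Helper functions for death offsets, normal or fire climb meshes and a wrapping counter are defined but not called here.
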(event `self.ReceiveBeginPlay`
  (set `CharacterMovementComponent.MaxWalkSpeed` (`self.Max Run Speed`) (`self.CharacterMovement`))
  (set `self.isWalking` true)
  (`self.K2_SetActorLocation` (`self.Start Position`))
  (`self.Move Mario To`))

(event `self.ReceiveTick`
  (params (DeltaSeconds :type "Float (single-precision)"))
  (if (`self.LoopEnded`)
    (`self.Idle/Walk Animation`)))

(event `Move Mario To`
  (`|AIMoveTo` self (`self.Destination`) null
    (:`OnSuccess`
      (`self.K2_SetActorLocation` (`self.Origin`))
      (`self.Move Mario To`))))

(event `Idle/Walk Animation`
  ;[1 0.3073 0.3073] Idle/Walk Animation
  (set `self.LoopEnded` false)
  (`self.Set Idle/ Walk Mario Model` "standing" :!label _label)
  (if (`self.isWalking`)
    (`self.Set Idle/ Walk Mario Model` "walk1" :!label _label_2)
    (`KismetSystemLibrary.Delay` (`self.RunDelta`))
    (if (`self.isWalking`)
      (`self.Set Idle/ Walk Mario Model` "walk2")
      (`KismetSystemLibrary.Delay` (`self.RunDelta`))
      (if (`self.isWalking`)
        (`self.Set Idle/ Walk Mario Model` "walk3")
        (`KismetSystemLibrary.Delay` (`self.RunDelta`))
        (if (`self.isWalking`)
          (goto _label_2)
          (else
            (goto _label)))
        (else
          (goto _label)))
      (else
        (goto _label)))
    (else
      (set `self.LoopEnded` true))))

(fn `DieAnimationDown`
  (params (Mesh :type "StaticMeshComponent Object Reference"))
  (returns (`New Location` :type "Vector Structure") (`New Rotation` :type "Rotator Structure"))
  (bind (_relativelocation_x _relativelocation_y _relativelocation_z) (`KismetMathLibrary.BreakVector` (`SceneComponent.RelativeLocation` Mesh)))
  (return (`KismetMathLibrary.MakeVector` _relativelocation_x _relativelocation_y (+ _relativelocation_z -200.0)) (`SceneComponent.RelativeRotation` Mesh)))

(fn `DieAnimationUp`
  (params (Mesh :type "StaticMeshComponent Object Reference"))
  (returns (`New Location` :type "Vector Structure") (`New Rotation` :type "Rotator Structure"))
  (bind (_relativerotation_roll _relativerotation_pitch _relativerotation_yaw) (`KismetMathLibrary.BreakRotator` (`SceneComponent.RelativeRotation` Mesh)))
  (bind (_relativelocation_x _relativelocation_y _relativelocation_z) (`KismetMathLibrary.BreakVector` (`SceneComponent.RelativeLocation` Mesh)))
  (return (`KismetMathLibrary.MakeVector` _relativelocation_x _relativelocation_y (+ _relativelocation_z 100.0)) (`KismetMathLibrary.MakeRotator` _relativerotation_roll (+ _relativerotation_pitch -180.0) _relativerotation_yaw)))

(fn `Increment Counter`
  (params (n :type Integer))
  (returns (newN :type Integer))
  (return (`KismetMathLibrary.FTrunc` (`KismetMathLibrary.FMod` (`KismetMathLibrary.Conv_IntToDouble` (+ n 1)) 4.0))))

(fn `Set Climb Mario Model`
  (params (isFire :type Boolean) (climbType :type String))
  (if isFire
    ;[1 0.3217 0.3018] Fire Mario
    (switch `string` climbType
      (:`climb1`
        (`StaticMeshComponent.SetStaticMesh` (`self.SM_Mario`) "/Game/Characters/Mario_Climb1_Fire/mario_climb1_fire.mario_climb1_fire"))
      (:`climb2`
        (`StaticMeshComponent.SetStaticMesh` (`self.SM_Mario`) "/Game/Characters/Mario_Climb2_Fire/mario_climb2_fire.mario_climb2_fire")))
    (else
      ;[0.6658 1 0.5117] Normal Mario
      (switch `string` climbType
        (:`climb1`
          (`StaticMeshComponent.SetStaticMesh` (`self.SM_Mario`) "/Game/Characters/Mario_Climb1/mario_climb1.mario_climb1"))
        (:`climb2`
          (`StaticMeshComponent.SetStaticMesh` (`self.SM_Mario`) "/Game/Characters/Mario_Climb2/mario_climb2.mario_climb2"))))))

(fn `Set Idle/ Walk Mario Model`
  (params (action :type String))
  ;[0.6658 1 0.5117] Normal Mario
  (switch `string` action
    (:`jump`
      (`StaticMeshComponent.SetStaticMesh` (`self.SM_Mario`) "/Game/Characters/Mario_Jump/mario_jump.mario_jump"))
    (:`standing`
      (`StaticMeshComponent.SetStaticMesh` (`self.SM_Mario`) "/Game/Characters/Mario_Standing/mario_standing.mario_standing"))
    (:`walk1`
      (`StaticMeshComponent.SetStaticMesh` (`self.SM_Mario`) "/Game/Characters/Mario_Walk1/mario_walk1.mario_walk1"))
    (:`walk2`
      (`StaticMeshComponent.SetStaticMesh` (`self.SM_Mario`) "/Game/Characters/Mario_Walk2/mario_walk2.mario_walk2"))
    (:`walk3`
      (`StaticMeshComponent.SetStaticMesh` (`self.SM_Mario`) "/Game/Characters/Mario_Walk3/mario_walk3.mario_walk3"))))

(fn `UserConstructionScript`)