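; BP_PointsSystem manages Mario's score, coins and lives, and handles his death.
; Point functions clamp score to a maximum, and the hundredth coin grants a life and resets the count.
; DeathHandler writes lives and default stats to the game instance, then shows a level intro, with world and level parsed from the level name.
; With no lives left, it restores initial values and shows Game Over.
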(fn `Add Points Brick Block`
  (params (`BP_Mario Ref` :type "/Game/Blueprints/BP_Mario Object Reference"))
  (locals (`Brick Block Points` :type Integer :default 50))
  (bind _formatted_points (`self.Check Points Limit` (+ (`/Game/Blueprints/BP_Mario.Score` `BP_Mario Ref`) (`local.Brick Block Points`))))
  (set `/Game/Blueprints/BP_Mario.Score` _formatted_points `BP_Mario Ref`))

(fn `Add Points Coin`
  (params (`BP_Mario Ref` :type "/Game/Blueprints/BP_Mario Object Reference"))
  (locals (`Coin Points` :type Integer :default 200))
  (bind _formatted_points (`self.Check Points Limit` (+ (`/Game/Blueprints/BP_Mario.Score` `BP_Mario Ref`) (`local.Coin Points`))))
  (set `/Game/Blueprints/BP_Mario.Score` _formatted_points `BP_Mario Ref`))

(fn `Add Points PowerUp`
  (params (`BP_Mario Ref` :type "/Game/Blueprints/BP_Mario Object Reference"))
  (locals (`PowerUp Points` :type Integer :default 1000))
  (bind _formatted_points (`self.Check Points Limit` (+ (`/Game/Blueprints/BP_Mario.Score` `BP_Mario Ref`) (`local.PowerUp Points`))))
  (set `/Game/Blueprints/BP_Mario.Score` _formatted_points `BP_Mario Ref`))

(fn `Check Points Limit`
  (params (Points :type Integer))
  (returns (`Formatted Points` :type Integer))
  (locals (`Maximum Score` :type Integer :default 9999999))
  (if (> Points (`local.Maximum Score`))
    (return (`local.Maximum Score`))
    (else
      (return Points))))

(fn `Death Handler`
  (params (`BP_Mario Ref` :type "/Game/Blueprints/BP_Mario Object Reference") (`BP_GameInst Ref` :type "/Game/Blueprints/BP_Game_Inst Object Reference"))
  (locals (BP_Mario :type "/Game/Blueprints/BP_Mario Object Reference"))
  (bind _output_get (set `local.BP_Mario` `BP_Mario Ref`))
  (`self.Set Default/Persisted Values` _output_get `BP_GameInst Ref`)
  (if (> (`/Game/Blueprints/BP_Mario.Lives` _output_get) 0)
    ;[1 0.3926 0.9902] Mario has lives left (show Level Intro Screen + restart level)
    (`WidgetLayoutLibrary.RemoveAllWidgets` null)
    (bind _returnvalue (`GameplayStatics.GetCurrentLevelName` null))
    (bind _returnvalue_2 (`|CreateWidget` "/Game/OtherUIs/WBP_LevelIntro.WBP_LevelIntro_C" (`GameplayStatics.GetPlayerController` null)))
    (bind (_lefts _rights) (`KismetStringLibrary.Split` (`KismetStringLibrary.GetSubstring` _returnvalue 3 3) "_"))
    (set `/Game/OtherUIs/WBP_LevelIntro.WorldNumber` (`KismetStringLibrary.Conv_StringToInt` _lefts) _returnvalue_2)
    (set `/Game/OtherUIs/WBP_LevelIntro.LevelNumber` (`KismetStringLibrary.Conv_StringToInt` _rights) _returnvalue_2)
    (set `/Game/OtherUIs/WBP_LevelIntro.LivesNumber` (`/Game/Blueprints/BP_Mario.Lives` (`local.BP_Mario`)) _returnvalue_2)
    (set `/Game/OtherUIs/WBP_LevelIntro.LevelName` _returnvalue _returnvalue_2)
    (`UserWidget.AddToViewport` _returnvalue_2 0)
    (else
      ;[0.4455 0.7411 1] Mario does not have lives left (show Time Up Screen/Game Over)
      (`self.Initialize Values` `BP_GameInst Ref`)
      (bind _returnvalue_3 (`|CreateWidget` "/Game/OtherUIs/WBP_GameOver.WBP_GameOver_C" (`GameplayStatics.GetPlayerController` null)))
      (`UserWidget.AddToViewport` _returnvalue_3 0))))

(fn `Decrease Lives Number`
  (params (`BP_Mario Ref` :type "/Game/Blueprints/BP_Mario Object Reference"))
  (set `/Game/Blueprints/BP_Mario.Lives` (- (`/Game/Blueprints/BP_Mario.Lives` `BP_Mario Ref`) 1) `BP_Mario Ref`))

(fn `Increase Coin Number`
  (params (`BP_Mario Ref` :type "/Game/Blueprints/BP_Mario Object Reference"))
  (bind _returnvalue (+ (`/Game/Blueprints/BP_Mario.Coins` `BP_Mario Ref`) 1))
  (if (== _returnvalue 100)
    ;[1 0.6335 0.3663] 100 coins = +1 life/0 coins
    (`self.Increase Lives Number` `BP_Mario Ref`)
    (set `/Game/Blueprints/BP_Mario.Coins` 0 `BP_Mario Ref`)
    (else
      ;[0.4794 0.8275 1] Less than 100 coins
      (set `/Game/Blueprints/BP_Mario.Coins` _returnvalue `BP_Mario Ref`))))

(fn `Increase Lives Number`
  (params (`BP_Mario Ref` :type "/Game/Blueprints/BP_Mario Object Reference"))
  (set `/Game/Blueprints/BP_Mario.Lives` (+ (`/Game/Blueprints/BP_Mario.Lives` `BP_Mario Ref`) 1) `BP_Mario Ref`))

(fn `Initialize Values`
  (params (`BP_GameInst Ref` :type "/Game/Blueprints/BP_Game_Inst Object Reference"))
  (locals (`Initial Lives` :type Integer :default 3) (`Initial Score` :type Integer) (`Initial Coins` :type Integer) (`Initial Timer` :type Integer :default 300))
  (set `/Game/Blueprints/BP_Game_Inst.isMarioFire` false `BP_GameInst Ref`)
  (set `/Game/Blueprints/BP_Game_Inst.MarioLives` (`local.Initial Lives`) `BP_GameInst Ref`)
  (set `/Game/Blueprints/BP_Game_Inst.MarioScore` (`local.Initial Score`) `BP_GameInst Ref`)
  (set `/Game/Blueprints/BP_Game_Inst.MarioCoins` (`local.Initial Coins`) `BP_GameInst Ref`)
  (set `/Game/Blueprints/BP_Game_Inst.TimeLeft` (`local.Initial Timer`) `BP_GameInst Ref`))

(fn `Set Default/Persisted Values`
  (params (`BP_Mario Ref` :type "/Game/Blueprints/BP_Mario Object Reference") (`BP_GameInst Ref` :type "/Game/Blueprints/BP_Game_Inst Object Reference"))
  (locals (`Default Score` :type Integer) (`Default Coins` :type Integer) (`Default Timer` :type Integer :default 300))
  (set `/Game/Blueprints/BP_Game_Inst.isMarioFire` false `BP_GameInst Ref`)
  (set `/Game/Blueprints/BP_Game_Inst.MarioLives` (`/Game/Blueprints/BP_Mario.Lives` `BP_Mario Ref`) `BP_GameInst Ref`)
  (set `/Game/Blueprints/BP_Game_Inst.MarioScore` (`local.Default Score`) `BP_GameInst Ref`)
  (set `/Game/Blueprints/BP_Game_Inst.MarioCoins` (`local.Default Coins`) `BP_GameInst Ref`)
  (set `/Game/Blueprints/BP_Game_Inst.TimeLeft` (`local.Default Timer`) `BP_GameInst Ref`))