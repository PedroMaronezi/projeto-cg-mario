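; BP_Fireball is a projectile actor, apparently for a Mario-style game, that kills Goombas and bounces a limited number of times.
; A self-calling event with a short Delay spins it continuously from BeginPlay, without Tick.
; Sphere hits destroy it on a Goomba, triggering that enemy's OnDie, or on a Koopa, which is left unaffected.
; Other hits increment a counter, and the fireball destroys itself once MaxHits is used up.
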(event `self.ReceiveBeginPlay`
  (`self.Rotation Animation`))

(event `Rotation Animation`
  ;[1 0.8349 0.3958] Rotation animation
  (`self.K2_AddActorLocalRotation` (struct :`Yaw` 9.0))
  (`KismetSystemLibrary.Delay` 0.0125)
  (`self.Rotation Animation`))

(event `self.Sphere.OnComponentHit`
  (params (HitComponent :type "PrimitiveComponent Object Reference") (OtherActor :type "Actor Object Reference") (OtherComp :type "PrimitiveComponent Object Reference") (NormalImpulse :type "Vector Structure") (Hit :type "HitResult Structure (by ref)"))
  ;[1 0.3801 0.2602] Fireball hits enemy/object
  (bind _asbp_goomba (cast `/Game/Blueprints/BP_Goomba` OtherActor)
    (:`then`
      (`self.K2_DestroyActor`)
      (`/Game/Blueprints/BP_Goomba.onDie` _asbp_goomba))
    (:`CastFailed`
      (cast `/Game/Blueprints/BP_Koopa` OtherActor
        (:`then`
          (`self.K2_DestroyActor`))
        (:`CastFailed`
          (if (< (`self.hits`) (`self.maxHits`))
            (set `self.hits` (+ (`self.hits`) 1))
            (else
              (`self.K2_DestroyActor`))))))))

(fn `UserConstructionScript`)