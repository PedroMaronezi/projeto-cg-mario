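; BP_1Up is a 1-Up pickup that stays hidden and non-colliding until a Show event fires, then destroys itself on overlapping BP_Mario.
; On show, it eases upward, then loops MoveComponentTo steps built from direction and falling state.
; Side colliders reverse its Y direction on overlap, while a bottom collider toggles falling as ground contact begins and ends.
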(event `self.ReceiveBeginPlay`
  (bind _1_up (`self.1_up`))
  (`ActorComponent.SetComponentTickEnabled` _1_up false)
  (`SceneComponent.SetVisibility` _1_up false false)
  (`PrimitiveComponent.SetCollisionEnabled` _1_up "NoCollision")
  (`PrimitiveComponent.SetCollisionEnabled` (`self.Collider_body`) "NoCollision")
  (`PrimitiveComponent.SetCollisionEnabled` (`self.Collider_bottom`) "NoCollision")
  (`PrimitiveComponent.SetCollisionEnabled` (`self.Collider_minusY`) "NoCollision")
  (`PrimitiveComponent.SetCollisionEnabled` (`self.Collider_plusY`) "NoCollision")
  (add `self.Show` (delegate `Show_Event`)))

(event `Show_Event`
  (bind _1_up (`self.1_up`))
  ;[1 0.9563 0.5144] Show 1-Up
  (`ActorComponent.SetComponentTickEnabled` _1_up true)
  (`SceneComponent.SetVisibility` _1_up true false)
  (`PrimitiveComponent.SetCollisionEnabled` _1_up "QueryAndPhysics")
  (`PrimitiveComponent.SetCollisionEnabled` (`self.Collider_body`) "QueryAndPhysics")
  (`PrimitiveComponent.SetCollisionEnabled` (`self.Collider_minusY`) "QueryAndPhysics")
  (`PrimitiveComponent.SetCollisionEnabled` (`self.Collider_plusY`) "QueryAndPhysics")
  (bind (_new_location _relative_rotation) (`self.goUp`))
  (`KismetSystemLibrary.MoveComponentTo` (`self.1_up`) _new_location _relative_rotation true true 1.0)
  (`PrimitiveComponent.SetCollisionEnabled` (`self.Collider_bottom`) "QueryAndPhysics")
  (`self.Move`))

(event `Move`
  (bind (_newlocation _relativerotation) (`self.MoveForward`))
  (`KismetSystemLibrary.MoveComponentTo` (`self.1_up`) _newlocation _relativerotation false false (`self.OverTime`))
  (`self.Move`))

(event `self.Collider_plusY.OnComponentBeginOverlap`
  (params (OverlappedComponent :type "PrimitiveComponent Object Reference") (OtherActor :type "Actor Object Reference") (OtherComp :type "PrimitiveComponent Object Reference") (OtherBodyIndex :type Integer) (bFromSweep :type Boolean) (SweepResult :type "HitResult Structure (by ref)"))
  (bind _direction (`self.Direction`))
  ;[1 0.6099 0.5096] Switch from +Y to -Y direction
  (if (== 1 _direction)
    (set `self.Direction` (* -1 _direction))))

(event `self.Collider_minusY.OnComponentBeginOverlap`
  (params (OverlappedComponent :type "PrimitiveComponent Object Reference") (OtherActor :type "Actor Object Reference") (OtherComp :type "PrimitiveComponent Object Reference") (OtherBodyIndex :type Integer) (bFromSweep :type Boolean) (SweepResult :type "HitResult Structure (by ref)"))
  (bind _direction (`self.Direction`))
  ;[0.5318 0.8373 1] Switch from -Y to +Y direction
  (if (== -1 _direction)
    (set `self.Direction` (* -1 _direction))))

(event `self.Collider_bottom.OnComponentBeginOverlap`
  (params (OverlappedComponent :type "PrimitiveComponent Object Reference") (OtherActor :type "Actor Object Reference") (OtherComp :type "PrimitiveComponent Object Reference") (OtherBodyIndex :type Integer) (bFromSweep :type Boolean) (SweepResult :type "HitResult Structure (by ref)"))
  ;[0.8002 0.5406 1] Fall
  (set `self.isFalling` 0))

(event `self.Collider_bottom.OnComponentEndOverlap`
  (params (OverlappedComponent :type "PrimitiveComponent Object Reference") (OtherActor :type "Actor Object Reference") (OtherComp :type "PrimitiveComponent Object Reference") (OtherBodyIndex :type Integer))
  ;[0.8002 0.5406 1] Fall
  (if (not (> (`KismetArrayLibrary.Array_Length` (`PrimitiveComponent.GetOverlappingActors` (`self.Collider_bottom`) null)) 1))
    (set `self.isFalling` 1)))

(event `self.Collider_body.OnComponentBeginOverlap`
  (params (OverlappedComponent :type "PrimitiveComponent Object Reference") (OtherActor :type "Actor Object Reference") (OtherComp :type "PrimitiveComponent Object Reference") (OtherBodyIndex :type Integer) (bFromSweep :type Boolean) (SweepResult :type "HitResult Structure (by ref)"))
  ;[0.461 1 0.5606] Interaction with Mario
  (cast `/Game/Blueprints/BP_Mario` OtherActor)
  (`self.K2_DestroyActor`))

(fn `GoUp`
  (returns (`New Location` :type "Vector Structure") (`Relative Rotation` :type "Rotator Structure"))
  (bind _1_up (`self.1_up`))
  (bind (_relativelocation_x _relativelocation_y _relativelocation_z) (`KismetMathLibrary.BreakVector` (`SceneComponent.RelativeLocation` _1_up)))
  (return (`KismetMathLibrary.MakeVector` _relativelocation_x _relativelocation_y (+ _relativelocation_z 160.0)) (`SceneComponent.RelativeRotation` _1_up)))

(fn `MoveForward`
  (returns (NewLocation :type "Vector Structure") (RelativeRotation :type "Rotator Structure"))
  (bind _1_up (`self.1_up`))
  (bind (_relativelocation_x _relativelocation_y _relativelocation_z) (`KismetMathLibrary.BreakVector` (`SceneComponent.RelativeLocation` _1_up)))
  (return (`KismetMathLibrary.MakeVector` _relativelocation_x (+ _relativelocation_y (* (`self.DistanceY`) (`self.Direction`))) (- _relativelocation_z (* (`self.DistanceZ`) (`self.isFalling`)))) (`SceneComponent.RelativeRotation` _1_up)))

(fn `UserConstructionScript`)