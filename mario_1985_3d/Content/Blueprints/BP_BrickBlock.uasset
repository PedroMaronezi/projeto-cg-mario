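; Mario-style brick block that reacts when BP_Mario overlaps it, as long as it still shows the Brick material.
; Coin blocks bounce, award points and spawn one animated coin at a time until empty; star blocks bounce and reveal their star.
; Empty blocks bounce for small Mario, judged by mesh scale, or award points and swap to the hidden physics-simulated BrickBlockDM for tall Mario before destroying the actor.
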(event `self.ReceiveBeginPlay`
  (bind _brick_block_dm (`self.brick_block_DM`))
  (`PrimitiveComponent.SetSimulatePhysics` _brick_block_dm false)
  (`ActorComponent.SetComponentTickEnabled` _brick_block_dm false)
  (`SceneComponent.SetVisibility` _brick_block_dm false false)
  (`PrimitiveComponent.SetCollisionEnabled` _brick_block_dm "NoCollision"))

(event `BounceAnimation`
  (bind _brick_block (`self.Brick_Block`))
  (bind _brick_block_2 (`self.Brick_Block`))
  ;[1 0.5601 0.5302] Bounce animation
  (bind (_newlocation _relativerotation) (`self.GoUp` _brick_block))
  (`KismetSystemLibrary.MoveComponentTo` _brick_block _newlocation _relativerotation true true (`self.JumpDuration`))
  (bind (_newlocation_2 _relativerotation_2) (`self.GoDown` _brick_block_2))
  (`KismetSystemLibrary.MoveComponentTo` _brick_block_2 _newlocation_2 _relativerotation_2 true true (`self.JumpDuration`)))

(event `self.ReceiveActorBeginOverlap`
  (params (OtherActor :type "Actor Object Reference"))
  (bind _brick_block (`self.Brick_Block`))
  (bind _brick_block_2 (`self.Brick_Block`))
  (bind _brick_block_3 (`self.Brick_Block`))
  (bind _brick_block_4 (`self.Brick_Block`))
  (bind _as_bp_mario (`self.As BP Mario`))
  (bind _brick_block_dm (`self.brick_block_DM`))
  (bind _brick_block_5 (`self.Brick_Block`))
  (bind _asbp_mario (cast `/Game/Blueprints/BP_Mario` OtherActor))
  (set `self.As BP Mario` _asbp_mario)
  (if (== (`PrimitiveComponent.GetMaterial` (`self.Brick_Block`) 0) "/Game/Blocks/materials/brick.brick")
    (if (`self.hasCoins`)
      ;[1 0.8357 0.5687] Block has coins
      (if (not (`self.isCoinAnimationPlaying`))
        (set `self.isCoinAnimationPlaying` true)
        (if (< (`self.n`) (`self.numCoins`))
          (`/Game/Functions/BP_UIHelperFunctions.Add Points Coin` _as_bp_mario)
          (`/Game/Functions/BP_UIHelperFunctions.Increase Coin Number` _as_bp_mario)
          (set `self.n` (+ (`self.n`) 1))
          (if (== (`self.n`) (`self.numCoins`))
            (`PrimitiveComponent.SetMaterial` (`self.Brick_Block`) 0 "/Game/Blocks/materials/opened.opened"))
          (`self.BounceAnimation`)
          (bind _returnvalue (`|SpawnActorFromClass` "/Game/Blueprints/BP_Coin.BP_Coin_C" (`SceneComponent.K2_GetComponentToWorld` (`self.CoinRef`)) "Undefined" "OverrideRootScale" null false true null))
          (`/Game/Blueprints/BP_Coin.JumpAnimation` _returnvalue)
          (if (`KismetSystemLibrary.IsValid` _returnvalue) :!label _label
            (`KismetSystemLibrary.Delay` 0.05)
            (goto _label)
            (else
              (set `self.isCoinAnimationPlaying` false)))))
      (elif (`self.hasStar`)
        ;[1 0.5892 0.4071] Block has star
        (`PrimitiveComponent.SetMaterial` (`self.Brick_Block`) 0 "/Game/Blocks/materials/opened.opened")
        (bind (_newlocation _relativerotation) (`self.GoUp` _brick_block_4))
        (`KismetSystemLibrary.MoveComponentTo` _brick_block_4 _newlocation _relativerotation true true (`self.JumpDuration`))
        (bind (_newlocation_2 _relativerotation_2) (`self.GoDown` _brick_block_2))
        (`KismetSystemLibrary.MoveComponentTo` _brick_block_2 _newlocation_2 _relativerotation_2 true true (`self.JumpDuration`))
        (`/Game/Blueprints/BP_Star.Show` (`self.StarRef`))
        (elif (`KismetMathLibrary.EqualExactly_VectorVector` (`SceneComponent.K2_GetComponentScale` (`/Game/Blueprints/BP_Mario.SM_Mario` _asbp_mario)) (1.0 1.0 1.0))
          ;[1 0.5233 0.4534] Empty block (small Mario)
          (`PrimitiveComponent.SetCollisionEnabled` (`self.Collision_Box`) "NoCollision")
          (bind (_newlocation_3 _relativerotation_3) (`self.GoUp` _brick_block_5))
          (`KismetSystemLibrary.MoveComponentTo` _brick_block_5 _newlocation_3 _relativerotation_3 true true (`self.JumpDuration`))
          (bind (_newlocation_4 _relativerotation_4) (`self.GoDown` _brick_block_3))
          (`KismetSystemLibrary.MoveComponentTo` _brick_block_3 _newlocation_4 _relativerotation_4 true true (`self.JumpDuration`))
          (`PrimitiveComponent.SetCollisionEnabled` (`self.Collision_Box`) "QueryAndPhysics")
          (else
            ;[1 0.6356 0.9941] Empty block (tall Mario)
            (`/Game/Functions/BP_UIHelperFunctions.Add Points Brick Block` (`self.As BP Mario`))
            (`ActorComponent.SetComponentTickEnabled` _brick_block false)
            (`SceneComponent.SetVisibility` _brick_block false false)
            (`PrimitiveComponent.SetCollisionEnabled` _brick_block "NoCollision")
            (`PrimitiveComponent.SetSimulatePhysics` _brick_block_dm true)
            (`ActorComponent.SetComponentTickEnabled` _brick_block_dm true)
            (`SceneComponent.SetVisibility` _brick_block_dm true false)
            (`PrimitiveComponent.SetCollisionEnabled` _brick_block_dm "QueryAndPhysics")
            (`KismetSystemLibrary.Delay` 7.0)
            (`self.K2_DestroyActor`)))))))

(fn `GoDown`
  (params (Mesh :type "SceneComponent Object Reference"))
  (returns (NewLocation :type "Vector Structure") (RelativeRotation :type "Rotator Structure"))
  (bind (_relativelocation_x _relativelocation_y _relativelocation_z) (`KismetMathLibrary.BreakVector` (`SceneComponent.RelativeLocation` Mesh)))
  (return (`KismetMathLibrary.MakeVector` _relativelocation_x _relativelocation_y (- _relativelocation_z (`self.JumpHeight`))) (`SceneComponent.RelativeRotation` Mesh)))

(fn `GoUp`
  (params (Mesh :type "SceneComponent Object Reference"))
  (returns (NewLocation :type "Vector Structure") (RelativeRotation :type "Rotator Structure"))
  (bind (_relativelocation_x _relativelocation_y _relativelocation_z) (`KismetMathLibrary.BreakVector` (`SceneComponent.RelativeLocation` Mesh)))
  (return (`KismetMathLibrary.MakeVector` _relativelocation_x _relativelocation_y (+ _relativelocation_z (`self.JumpHeight`))) (`SceneComponent.RelativeRotation` Mesh)))

(fn `UserConstructionScript`)