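; Fire Flower power-up that starts hidden and, once collected by BP_Mario, calls GetFireFlower on him and destroys itself.
; BeginPlay disables the flower's visibility, tick and collision, then binds to a Show event that restores them and eases the flower upward.
; Showing also starts a self-calling Animation event that loops through flower materials with timed delays, though the fourth is immediately replaced by the first.
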(event `self.ReceiveBeginPlay`
  (bind _fire_flower (`self.fire_flower`))
  (`ActorComponent.SetComponentTickEnabled` _fire_flower false)
  (`SceneComponent.SetVisibility` _fire_flower false false)
  (`PrimitiveComponent.SetCollisionEnabled` _fire_flower "NoCollision")
  (`PrimitiveComponent.SetCollisionEnabled` (`self.Box`) "NoCollision")
  (add `self.Show` (delegate `Show_Event`)))

(event `Show_Event`
  (bind _fire_flower (`self.fire_flower`))
  ;[1 0.3057 0.6265] Show Fire Flower
  (`ActorComponent.SetComponentTickEnabled` _fire_flower true)
  (`SceneComponent.SetVisibility` _fire_flower true false)
  (`PrimitiveComponent.SetCollisionEnabled` _fire_flower "QueryAndPhysics")
  (`PrimitiveComponent.SetCollisionEnabled` (`self.Box`) "QueryAndPhysics")
  (`self.Animation`)
  (bind (_new_location _relative_rotation) (`self.goUp`))
  (`KismetSystemLibrary.MoveComponentTo` (`self.fire_flower`) _new_location _relative_rotation true true 0.5))

(event `Animation`
  ;[0.542 0.8687 1] Color Animation
  (`PrimitiveComponent.SetMaterial` (`self.fire_flower`) 0 "/Game/Items/Fireflower/Material_Fire_Flower_1.Material_Fire_Flower_1")
  (`KismetSystemLibrary.Delay` (`self.AnimationDelta`))
  (`PrimitiveComponent.SetMaterial` (`self.fire_flower`) 0 "/Game/Items/Fireflower/Material_Fire_Flower_2.Material_Fire_Flower_2")
  (`KismetSystemLibrary.Delay` (`self.AnimationDelta`))
  (`PrimitiveComponent.SetMaterial` (`self.fire_flower`) 0 "/Game/Items/Fireflower/Material_Fire_Flower_3.Material_Fire_Flower_3")
  (`KismetSystemLibrary.Delay` (`self.AnimationDelta`))
  (`PrimitiveComponent.SetMaterial` (`self.fire_flower`) 0 "/Game/Items/Fireflower/Material_Fire_Flower_4.Material_Fire_Flower_4")
  (`self.Animation`))

(event `self.Box.OnComponentBeginOverlap`
  (params (OverlappedComponent :type "PrimitiveComponent Object Reference") (OtherActor :type "Actor Object Reference") (OtherComp :type "PrimitiveComponent Object Reference") (OtherBodyIndex :type Integer) (bFromSweep :type Boolean) (SweepResult :type "HitResult Structure (by ref)"))
  ;[1 0.5692 0.3873] Fire Flower interaction with Mario
  (bind _asbp_mario (cast `/Game/Blueprints/BP_Mario` OtherActor))
  (`self.K2_DestroyActor`)
  (`/Game/Blueprints/BP_Mario.Get Fire Flower` _asbp_mario))

(fn `goUp`
  (returns (`New Location` :type "Vector Structure") (`Relative Rotation` :type "Rotator Structure"))
  (bind _fire_flower (`self.fire_flower`))
  (bind (_relativelocation_x _relativelocation_y _relativelocation_z) (`KismetMathLibrary.BreakVector` (`SceneComponent.RelativeLocation` _fire_flower)))
  (return (`KismetMathLibrary.MakeVector` _relativelocation_x _relativelocation_y (+ _relativelocation_z 160.0)) (`SceneComponent.RelativeRotation` _fire_flower)))

(fn `UserConstructionScript`)