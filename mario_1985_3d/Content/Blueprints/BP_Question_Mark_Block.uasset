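; Mario-style question mark block that, when Mario overlaps its box, bounces and releases either coins or an item.
; A timeline animates the metallic parameter on its dynamic materials, and the side material doubles as the still-active check until swapped for Opened.
; Coin blocks spawn a jumping coin per hit up to a limit.
; Item blocks reveal themselves if invisible, then show a 1-Up, or a mushroom or fire flower depending on Mario's capsule scale.
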(event `self.ReceiveBeginPlay`
  (bind _question_mark_block (`self.question_mark_block`))
  (if (`self.isInvisible`)
    (`SceneComponent.SetVisibility` (`self.question_mark_block`) false false))
  ;[1 0.5816 0.2731] Metallic Property Animation
  (bind _returnvalue (`PrimitiveComponent.CreateDynamicMaterialInstance` _question_mark_block 0 "/Game/Blocks/models/question_mark_block/Material_Question_Mark_Sides.Material_Question_Mark_Sides" "None"))
  (set `self.MaterialRef` _returnvalue)
  (bind _returnvalue_2 (`PrimitiveComponent.CreateDynamicMaterialInstance` _question_mark_block 1 "/Game/Blocks/models/question_mark_block/Material_Question_Mark_Top.Material_Question_Mark_Top" "None"))
  (bind (_direction _metallic_value) (`Timeline|Timeline_0`)
    (:`Update`
      (`MaterialInstanceDynamic.SetScalarParameterValue` _returnvalue "Metal" _metallic_value)
      (`MaterialInstanceDynamic.SetScalarParameterValue` _returnvalue_2 "Metal" _metallic_value))))

(event `BounceAnimation`
  ;[1 0.5104 0.5104] Bounce animation
  (bind (_newlocation _relativerotation) (`self.GoUp`))
  (`KismetSystemLibrary.MoveComponentTo` (`self.question_mark_block`) _newlocation _relativerotation true true (`self.JumpDuration`))
  (bind (_newlocation_2 _relativerotation_2) (`self.GoDown`))
  (`KismetSystemLibrary.MoveComponentTo` (`self.question_mark_block`) _newlocation_2 _relativerotation_2 true true (`self.JumpDuration`)))

(event `self.Box.OnComponentBeginOverlap`
  (params (OverlappedComponent :type "PrimitiveComponent Object Reference") (OtherActor :type "Actor Object Reference") (OtherComp :type "PrimitiveComponent Object Reference") (OtherBodyIndex :type Integer) (bFromSweep :type Boolean) (SweepResult :type "HitResult Structure (by ref)"))
  (bind _asbp_mario (cast `/Game/Blueprints/BP_Mario` OtherActor))
  (if (== (`self.MaterialRef`) (`PrimitiveComponent.GetMaterial` (`self.question_mark_block`) 0))
    (if (`self.hasCoins`)
      ;[1 0.8357 0.5687] Block has coins
      (if (< (`self.n`) (`self.numCoins`))
        (set `self.n` (+ (`self.n`) 1))
        (if (== (`self.n`) (`self.numCoins`))
          (`PrimitiveComponent.SetMaterial` (`self.question_mark_block`) 0 "/Game/Blocks/materials/opened.opened"))
        (`self.BounceAnimation`)
        (bind _returnvalue (`|SpawnActorFromClass` "/Game/Blueprints/BP_Coin.BP_Coin_C" (`SceneComponent.K2_GetComponentToWorld` (`self.CoinRef`)) "Undefined" "OverrideRootScale" null false true null))
        (`/Game/Blueprints/BP_Coin.JumpAnimation` _returnvalue))
      (else
        ;[0.5342 0.92 1] Block has power-up
        (`SceneComponent.SetVisibility` (`self.question_mark_block`) true false)
        (`PrimitiveComponent.SetMaterial` (`self.question_mark_block`) 0 "/Game/Blocks/materials/opened.opened")
        (bind (_newlocation _relativerotation) (`self.GoUp`))
        (`KismetSystemLibrary.MoveComponentTo` (`self.question_mark_block`) _newlocation _relativerotation true true (`self.JumpDuration`))
        (bind (_newlocation_2 _relativerotation_2) (`self.GoDown`))
        (`KismetSystemLibrary.MoveComponentTo` (`self.question_mark_block`) _newlocation_2 _relativerotation_2 true true (`self.JumpDuration`))
        (if (`self.has1Up`)
          (`/Game/Blueprints/BP_1Up.Show` (`self.1UpRef`))
          (elif (`self.hasPowerup`)
            (if (`KismetMathLibrary.EqualExactly_VectorVector` (`SceneComponent.K2_GetComponentScale` (`Character.CapsuleComponent` _asbp_mario)) (1.0 1.0 1.0))
              (`/Game/Blueprints/BP_Mushroom.Show` (`self.MushroomRef`))
              (else
                (`/Game/Blueprints/BP_Fireflower.Show` (`self.FireFlowerRef`))))))))))

(fn `goDown`
  (returns (NewLocation :type "Vector Structure") (RelativeRotation :type "Rotator Structure"))
  (bind _question_mark_block (`self.question_mark_block`))
  (bind (_relativelocation_x _relativelocation_y _relativelocation_z) (`KismetMathLibrary.BreakVector` (`SceneComponent.RelativeLocation` _question_mark_block)))
  (return (`KismetMathLibrary.MakeVector` _relativelocation_x _relativelocation_y (- _relativelocation_z (`self.JumpHeight`))) (`SceneComponent.RelativeRotation` _question_mark_block)))

(fn `goUp`
  (returns (NewLocation :type "Vector Structure") (RelativeRotation :type "Rotator Structure"))
  (bind _question_mark_block (`self.question_mark_block`))
  (bind (_relativelocation_x _relativelocation_y _relativelocation_z) (`KismetMathLibrary.BreakVector` (`SceneComponent.RelativeLocation` _question_mark_block)))
  (return (`KismetMathLibrary.MakeVector` _relativelocation_x _relativelocation_y (+ _relativelocation_z (`self.JumpHeight`))) (`SceneComponent.RelativeRotation` _question_mark_block)))

(fn `UserConstructionScript`)