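; BP_Goomba is a Mario-style Goomba enemy that patrols, turns 180 degrees when its front collider hits something and falls when its foot collider loses ground.
; Movement chains MoveComponentTo steps on the mesh, while Tick drives a two-mesh swap walk animation.
; Body contact calls Mario's OnHit, or kills the Goomba if Mario has a star.
; Head contact from Mario squashes it, then destroys it after a delay.
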(event `self.ReceiveBeginPlay`
  (`self.MoveMob`))

(event `self.ReceiveTick`
  (params (DeltaSeconds :type "Float (single-precision)"))
  (if (`self.Loop Ended`)
    (`self.WalkAnimation`)))

(event `MoveMob`
  (bind _sm_goomba (`self.SM_Goomba`))
  (bind _sm_goomba_2 (`self.SM_Goomba`))
  ;[0.146 0.5729 1] Move Mob
  (bind (_new_position _new_rotation) (`self.GoForward` _sm_goomba))
  (`KismetSystemLibrary.MoveComponentTo` _sm_goomba _new_position _new_rotation false false (`self.OverTime`) :!label _label)
  (if (`self.isFlipping`)
    (set `self.Direction` (* -1 (`self.Direction`)))
    (bind _new_rotation_2 (`self.Flip` 180.0 _sm_goomba_2))
    (`KismetSystemLibrary.MoveComponentTo` _sm_goomba_2 (`SceneComponent.RelativeLocation` _sm_goomba_2) _new_rotation_2 false false (`self.FlipTime`))
    (set `self.isFlipping` false)
    (`self.MoveMob`)
    (else
      (`self.MoveMob`))))

(event `self.Collider_Front.OnComponentBeginOverlap`
  (params (OverlappedComponent :type "PrimitiveComponent Object Reference") (OtherActor :type "Actor Object Reference") (OtherComp :type "PrimitiveComponent Object Reference") (OtherBodyIndex :type Integer) (bFromSweep :type Boolean) (SweepResult :type "HitResult Structure (by ref)"))
  ;[0.146 0.5729 1] Move Mob
  (set `self.isFlipping` true)
  (goto _label :!via `Stop`))

(event `self.Collider_Foot.OnComponentEndOverlap`
  (params (OverlappedComponent :type "PrimitiveComponent Object Reference") (OtherActor :type "Actor Object Reference") (OtherComp :type "PrimitiveComponent Object Reference") (OtherBodyIndex :type Integer))
  ;[0.146 0.5729 1] Move Mob
  (if (not (> (`KismetArrayLibrary.Array_Length` (`PrimitiveComponent.GetOverlappingActors` (`self.Collider_Foot`) null)) 1))
    (set `self.isFalling` 1)))

(event `self.Collider_Foot.OnComponentBeginOverlap`
  (params (OverlappedComponent :type "PrimitiveComponent Object Reference") (OtherActor :type "Actor Object Reference") (OtherComp :type "PrimitiveComponent Object Reference") (OtherBodyIndex :type Integer) (bFromSweep :type Boolean) (SweepResult :type "HitResult Structure (by ref)"))
  ;[0.146 0.5729 1] Move Mob
  (set `self.isFalling` 0))

(event `WalkAnimation`
  ;[1 0.9993 0.001249] Walking Animation
  (set `self.Loop Ended` false)
  (`StaticMeshComponent.SetStaticMesh` (`self.SM_Goomba`) "/Game/Characters/Goomba_1/goomba_1.goomba_1")
  (`KismetSystemLibrary.Delay` (`self.Delay Time`))
  (`StaticMeshComponent.SetStaticMesh` (`self.SM_Goomba`) "/Game/Characters/Goomba_2/goomba_2.goomba_2")
  (`KismetSystemLibrary.Delay` (`self.Delay Time`))
  (set `self.Loop Ended` true))

(event `self.Collider_Body.OnComponentBeginOverlap`
  (params (OverlappedComponent :type "PrimitiveComponent Object Reference") (OtherActor :type "Actor Object Reference") (OtherComp :type "PrimitiveComponent Object Reference") (OtherBodyIndex :type Integer) (bFromSweep :type Boolean) (SweepResult :type "HitResult Structure (by ref)"))
  (bind _asbp_mario (cast `/Game/Blueprints/BP_Mario` OtherActor))
  (if (`self.isDead`)
    _
    (elif (`/Game/Blueprints/BP_Mario.isStar` _asbp_mario)
      (`self.onDie`)
      (else
        (`/Game/Blueprints/BP_Mario.OnHit` _asbp_mario)))))

(event `self.Collider_Head.OnComponentBeginOverlap`
  (params (OverlappedComponent :type "PrimitiveComponent Object Reference") (OtherActor :type "Actor Object Reference") (OtherComp :type "PrimitiveComponent Object Reference") (OtherBodyIndex :type Integer) (bFromSweep :type Boolean) (SweepResult :type "HitResult Structure (by ref)"))
  (cast `/Game/Blueprints/BP_Mario` OtherActor)
  (`self.onDie`))

(event `onDie`
  (set `self.isDead` true)
  (`self.DieAnimation` (`self.SM_Goomba`))
  (`KismetSystemLibrary.Delay` 1.0)
  (`self.K2_DestroyActor`))

(fn `DieAnimation`
  (params (Mesh :type "StaticMeshComponent Object Reference"))
  (bind (_relativescale3d_x _relativescale3d_y) (`KismetMathLibrary.BreakVector` (`SceneComponent.RelativeScale3D` Mesh)))
  (`SceneComponent.SetRelativeScale3D` Mesh (`KismetMathLibrary.MakeVector` _relativescale3d_x _relativescale3d_y 0.2))
  (return))

(fn `Flip`
  (params (Degree :type "Float (double-precision)") (Mesh :type "StaticMeshComponent Object Reference"))
  (returns (`New Rotation` :type "Rotator Structure"))
  (bind (_relativerotation_roll _relativerotation_pitch _relativerotation_yaw) (`KismetMathLibrary.BreakRotator` (`SceneComponent.RelativeRotation` Mesh)))
  (return (`KismetMathLibrary.MakeRotator` _relativerotation_roll _relativerotation_pitch (+ Degree _relativerotation_yaw))))

(fn `GoBackward`
  (params (Mesh :type "StaticMeshComponent Object Reference"))
  (returns (`New Position` :type "Vector Structure") (`New Rotation` :type "Rotator Structure"))
  (bind (_relativelocation_x _relativelocation_y _relativelocation_z) (`KismetMathLibrary.BreakVector` (`SceneComponent.RelativeLocation` Mesh)))
  (return (`KismetMathLibrary.MakeVector` _relativelocation_x (- (`self.MoveDistance`) _relativelocation_y) _relativelocation_z) (`SceneComponent.RelativeRotation` Mesh)))

(fn `GoForward`
  (params (Mesh :type "StaticMeshComponent Object Reference"))
  (returns (`New Position` :type "Vector Structure") (`New Rotation` :type "Rotator Structure"))
  (bind (_relativelocation_x _relativelocation_y _relativelocation_z) (`KismetMathLibrary.BreakVector` (`SceneComponent.RelativeLocation` Mesh)))
  (return (`KismetMathLibrary.MakeVector` _relativelocation_x (+ (* (`self.DistanceY`) (`self.Direction`)) _relativelocation_y) (- _relativelocation_z (* (`self.DistanceZ`) (`self.isFalling`)))) (`SceneComponent.RelativeRotation` Mesh)))

(fn `UserConstructionScript`)