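; Level-transition trigger that loads a named level when Mario enters its box, or crouches inside it when HasToCrounch is set.
; Before loading, it saves the spawn transform with Mario's mesh scale and his fire state to BP_Game_Inst.
; The crouch path polls overlaps on Tick, doubles the saved Z scale, calls DownPipe and delays the load.
; The plain path loads immediately on begin overlap.
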(event `self.ReceiveTick`
  (params (DeltaSeconds :type "Float (single-precision)"))
  (bind (_spawnlocation_location _spawnlocation_rotation) (`KismetMathLibrary.BreakTransform` (`self.spawnLocation`)))
  (bind _overlappingactors (`PrimitiveComponent.GetOverlappingActors` (`self.Box`) "/Game/Blueprints/BP_Mario.BP_Mario_C"))
  ;[1 0.3022 0.1521] Change Level when Crouching
  (if (`self.hasToCrounch`)
    (if (> (`KismetArrayLibrary.Array_Length` _overlappingactors) 0)
      (bind _asbp_mario (cast `/Game/Blueprints/BP_Mario` (`|GetArrayItem` _overlappingactors)))
      (if (`/Game/Blueprints/BP_Mario.isCrouching` _asbp_mario)
        (bind _asbp_game_inst (cast `/Game/Blueprints/BP_Game_Inst` (`GameplayStatics.GetGameInstance`)))
        (bind _returnvalue (`SceneComponent.K2_GetComponentToWorld` (`/Game/Blueprints/BP_Mario.SM_Mario` _asbp_mario)))
        (set `/Game/Blueprints/BP_Game_Inst.spawnLocation` (`KismetMathLibrary.MakeTransform` _spawnlocation_location _spawnlocation_rotation (`KismetMathLibrary.MakeVector` (.x (.scale _returnvalue)) (.y (.scale _returnvalue)) (/ (.z (.scale _returnvalue)) 0.5))) _asbp_game_inst)
        (set `/Game/Blueprints/BP_Game_Inst.isMarioFire` (`/Game/Blueprints/BP_Mario.isFire` _asbp_mario) _asbp_game_inst)
        (`/Game/Blueprints/BP_Mario.Down Pipe` _asbp_mario)
        (`KismetSystemLibrary.Delay` 1.6)
        (`GameplayStatics.OpenLevel` (`self.Level Name`))))))

(event `self.Box.OnComponentBeginOverlap`
  (params (OverlappedComponent :type "PrimitiveComponent Object Reference") (OtherActor :type "Actor Object Reference") (OtherComp :type "PrimitiveComponent Object Reference") (OtherBodyIndex :type Integer) (bFromSweep :type Boolean) (SweepResult :type "HitResult Structure (by ref)"))
  (bind (_spawnlocation_location _spawnlocation_rotation) (`KismetMathLibrary.BreakTransform` (`self.spawnLocation`)))
  ;[0.07409 0.7375 1] Change Level
  (bind _asbp_mario (cast `/Game/Blueprints/BP_Mario` OtherActor))
  (if (not (`self.hasToCrounch`))
    (bind _asbp_game_inst (cast `/Game/Blueprints/BP_Game_Inst` (`GameplayStatics.GetGameInstance`)))
    (bind (_returnvalue_location _returnvalue_rotation _returnvalue_scale) (`KismetMathLibrary.BreakTransform` (`SceneComponent.K2_GetComponentToWorld` (`/Game/Blueprints/BP_Mario.SM_Mario` _asbp_mario))))
    (set `/Game/Blueprints/BP_Game_Inst.spawnLocation` (`KismetMathLibrary.MakeTransform` _spawnlocation_location _spawnlocation_rotation _returnvalue_scale) _asbp_game_inst)
    (set `/Game/Blueprints/BP_Game_Inst.isMarioFire` (`/Game/Blueprints/BP_Mario.isFire` _asbp_mario) _asbp_game_inst)
    (`GameplayStatics.OpenLevel` (`self.Level Name`))))

(fn `UserConstructionScript`)