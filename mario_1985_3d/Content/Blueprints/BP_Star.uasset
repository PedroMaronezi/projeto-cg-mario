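; BP_Star is a Super Star pickup that grants BP_Mario invincibility on overlap and destroys itself.
; It starts hidden with collision and physics off until the event bound through BindEventToShow fires.
; Showing it eases the Sphere upward, then enables physics and launches it with a fixed velocity.
; A self-calling Animation event with delays cycles the Star mesh's materials for a color-flashing effect.
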(event `self.ReceiveBeginPlay`
  (bind _sphere (`self.Sphere`))
  (bind _star (`self.star`))
  (`ActorComponent.SetComponentTickEnabled` _sphere false)
  (`SceneComponent.SetVisibility` _sphere false false)
  (`PrimitiveComponent.SetSimulatePhysics` _sphere false)
  (`PrimitiveComponent.SetCollisionEnabled` (`self.Box`) "NoCollision")
  (`ActorComponent.SetComponentTickEnabled` _star false)
  (`SceneComponent.SetVisibility` _star false false)
  (add `self.Show` (delegate `Show_Event`)))

(event `Show_Event`
  (bind _sphere (`self.Sphere`))
  (bind _sphere_2 (`self.Sphere`))
  (bind _star (`self.star`))
  ;[1 0.4177 0.1958] Show Star
  (`ActorComponent.SetComponentTickEnabled` _sphere true)
  (`SceneComponent.SetVisibility` _sphere true false)
  (`PrimitiveComponent.SetCollisionEnabled` (`self.Box`) "QueryAndPhysics")
  (`ActorComponent.SetComponentTickEnabled` _star true)
  (`SceneComponent.SetVisibility` _star true false)
  (`self.Animation`)
  (bind (_new_location _relative_rotation) (`self.goUp`))
  (`KismetSystemLibrary.MoveComponentTo` _sphere_2 _new_location _relative_rotation true true 0.5)
  (`PrimitiveComponent.SetSimulatePhysics` _sphere_2 true)
  (`PrimitiveComponent.SetPhysicsLinearVelocity` (`self.Sphere`) (0.0 -700.0 400.0) false "None"))

(event `Animation`
  ;[1 0.8364 0.3739] Color Animation
  (`PrimitiveComponent.SetMaterial` (`self.star`) 0 "/Game/Items/Star/Material_Star_1.Material_Star_1")
  (`KismetSystemLibrary.Delay` (`self.AnimationDelta`))
  (`PrimitiveComponent.SetMaterial` (`self.star`) 0 "/Game/Items/Star/Material_Star_2.Material_Star_2")
  (`KismetSystemLibrary.Delay` (`self.AnimationDelta`))
  (`PrimitiveComponent.SetMaterial` (`self.star`) 0 "/Game/Items/Star/Material_Star_3.Material_Star_3")
  (`KismetSystemLibrary.Delay` (`self.AnimationDelta`))
  (`PrimitiveComponent.SetMaterial` (`self.star`) 0 "/Game/Items/Star/Material_Star_4.Material_Star_4")
  (`self.Animation`))

(event `self.Box.OnComponentBeginOverlap`
  (params (OverlappedComponent :type "PrimitiveComponent Object Reference") (OtherActor :type "Actor Object Reference") (OtherComp :type "PrimitiveComponent Object Reference") (OtherBodyIndex :type Integer) (bFromSweep :type Boolean) (SweepResult :type "HitResult Structure (by ref)"))
  ;[0.5103 0.9901 1] Star interaction with Mario
  (bind _asbp_mario (cast `/Game/Blueprints/BP_Mario` OtherActor))
  (`self.K2_DestroyActor`)
  (`/Game/Blueprints/BP_Mario.Get Invincibility` _asbp_mario))

(fn `goUp`
  (returns (`New Location` :type "Vector Structure") (`Relative Rotation` :type "Rotator Structure"))
  (bind _sphere (`self.Sphere`))
  (bind (_relativelocation_x _relativelocation_y _relativelocation_z) (`KismetMathLibrary.BreakVector` (`SceneComponent.RelativeLocation` _sphere)))
  (return (`KismetMathLibrary.MakeVector` _relativelocation_x _relativelocation_y (+ _relativelocation_z 160.0)) (`SceneComponent.RelativeRotation` _sphere)))

(fn `UserConstructionScript`)