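; Koopa enemy that walks, hurts Mario on contact, and becomes a fast spinning shell when stomped.
; MoveMob chains relative MoveComponentTo steps, with foot overlaps toggling falling, front overlaps flipping the walker and shell overlaps reversing the shell.
; Tick drives a two-mesh walk cycle, or swaps in the shell mesh and speeds up movement once dead.
; The shell kills Goombas and hurts Mario; star Mario triggers a flip-and-drop death, then destruction.
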(event `self.ReceiveBeginPlay`
  (`self.Move Mob`))

(event `self.ReceiveTick`
  (params (DeltaSeconds :type "Float (single-precision)"))
  (if (`self.Loop Ended`)
    (`self.WalkAnimation`)))

(event `Move Mob`
  (bind _sm_koopa (`self.SM_Koopa`))
  (bind _sm_koopa_2 (`self.SM_Koopa`))
  (bind (_new_position _new_rotation) (`self.GoForward` _sm_koopa_2))
  (`KismetSystemLibrary.MoveComponentTo` _sm_koopa_2 _new_position _new_rotation false false (`self.OverTime`) :!label _label)
  (if (`self.isFlipping`)
    (set `self.Direction` (* -1 (`self.Direction`)))
    (bind _new_rotation_2 (`self.Flip` 180.0 _sm_koopa))
    (`KismetSystemLibrary.MoveComponentTo` _sm_koopa (`SceneComponent.RelativeLocation` _sm_koopa) _new_rotation_2 false false (`self.FlipTime`))
    (set `self.isFlipping` false)
    (`self.Move Mob`)
    (elif (`self.shellColided`)
      (set `self.Direction` (* -1 (`self.Direction`)))
      (set `self.shellColided` false)
      (`self.Move Mob`)
      (else
        (`self.Move Mob`)))))

(event `self.Collider_Front.OnComponentBeginOverlap`
  (params (OverlappedComponent :type "PrimitiveComponent Object Reference") (OtherActor :type "Actor Object Reference") (OtherComp :type "PrimitiveComponent Object Reference") (OtherBodyIndex :type Integer) (bFromSweep :type Boolean) (SweepResult :type "HitResult Structure (by ref)"))
  (if (not (`self.isDead`))
    (set `self.isFlipping` true)
    (goto _label :!via `Stop`)))

(event `self.Collider_Shell.OnComponentBeginOverlap`
  (params (OverlappedComponent :type "PrimitiveComponent Object Reference") (OtherActor :type "Actor Object Reference") (OtherComp :type "PrimitiveComponent Object Reference") (OtherBodyIndex :type Integer) (bFromSweep :type Boolean) (SweepResult :type "HitResult Structure (by ref)"))
  (if (`self.isDead`)
    (cast `/Game/Blueprints/BP_MobWall` OtherActor
      (:`CastFailed`
        (set `self.shellColided` true)))))

(event `self.Collider_Foot.OnComponentBeginOverlap`
  (params (OverlappedComponent :type "PrimitiveComponent Object Reference") (OtherActor :type "Actor Object Reference") (OtherComp :type "PrimitiveComponent Object Reference") (OtherBodyIndex :type Integer) (bFromSweep :type Boolean) (SweepResult :type "HitResult Structure (by ref)"))
  (set `self.isFalling` 0))

(event `self.Collider_Foot.OnComponentEndOverlap`
  (params (OverlappedComponent :type "PrimitiveComponent Object Reference") (OtherActor :type "Actor Object Reference") (OtherComp :type "PrimitiveComponent Object Reference") (OtherBodyIndex :type Integer))
  (cast `/Game/Blueprints/BP_MobWall` OtherActor
    (:`CastFailed`
      (if (not (> (`KismetArrayLibrary.Array_Length` (`PrimitiveComponent.GetOverlappingActors` (`self.Collider_Foot`) null)) 1))
        (set `self.isFalling` 1)))))

(event `WalkAnimation`
  ;[1 0.8331 0] Walk Animation
  (if (`self.isDead`)
    (`StaticMeshComponent.SetStaticMesh` (`self.SM_Koopa`) "/Game/Characters/Shell/shell.shell")
    (set `self.OverTime` 0.05)
    (set `self.FlipTime` 0.3)
    (else
      (set `self.Loop Ended` false)
      (`StaticMeshComponent.SetStaticMesh` (`self.SM_Koopa`) "/Game/Characters/Koopa_1/koopa_1.koopa_1")
      (`KismetSystemLibrary.Delay` (`self.Delay Time`))
      (`StaticMeshComponent.SetStaticMesh` (`self.SM_Koopa`) "/Game/Characters/Koopa_2/koopa_2.koopa_2")
      (`KismetSystemLibrary.Delay` (`self.Delay Time`))
      (set `self.Loop Ended` true))))

(event `self.Collider_Dead_Body.OnComponentBeginOverlap`
  (params (OverlappedComponent :type "PrimitiveComponent Object Reference") (OtherActor :type "Actor Object Reference") (OtherComp :type "PrimitiveComponent Object Reference") (OtherBodyIndex :type Integer) (bFromSweep :type Boolean) (SweepResult :type "HitResult Structure (by ref)"))
  ;[1 0.07432 0.3682] Dead Body Interaction
  (bind _asbp_mario (cast `/Game/Blueprints/BP_Mario` OtherActor)
    (:`then`
      (if (`self.isDead`)
        (if (`/Game/Blueprints/BP_Mario.isStar` _asbp_mario)
          (`self.onDieByHit`)
          (else
            (`/Game/Blueprints/BP_Mario.OnHit` _asbp_mario)))))
    (:`CastFailed`
      (bind _asbp_goomba (cast `/Game/Blueprints/BP_Goomba` OtherActor))
      (if (`self.isDead`)
        (`/Game/Blueprints/BP_Goomba.onDie` _asbp_goomba)))))

(event `self.Collider_Body.OnComponentBeginOverlap`
  (params (OverlappedComponent :type "PrimitiveComponent Object Reference") (OtherActor :type "Actor Object Reference") (OtherComp :type "PrimitiveComponent Object Reference") (OtherBodyIndex :type Integer) (bFromSweep :type Boolean) (SweepResult :type "HitResult Structure (by ref)"))
  ;[0.822 0.4034 1] Kill Mario / Die to Mario Star
  (bind _asbp_mario (cast `/Game/Blueprints/BP_Mario` OtherActor))
  (if (`self.isDead`)
    _
    (elif (`/Game/Blueprints/BP_Mario.isStar` _asbp_mario)
      (`self.onDieByHit`)
      (else
        (`/Game/Blueprints/BP_Mario.OnHit` _asbp_mario)))))

(event `On Die`
  ;[1 1 1] Die
  (set `self.isDead` true)
  (set `self.isRotating` 1))

(event `self.Collider_Head.OnComponentBeginOverlap`
  (params (OverlappedComponent :type "PrimitiveComponent Object Reference") (OtherActor :type "Actor Object Reference") (OtherComp :type "PrimitiveComponent Object Reference") (OtherBodyIndex :type Integer) (bFromSweep :type Boolean) (SweepResult :type "HitResult Structure (by ref)"))
  ;[1 0.04144 0.06134] Kill Koopa
  (if (not (`self.isDead`))
    (bind _asbp_mario (cast `/Game/Blueprints/BP_Mario` OtherActor))
    (`self.On Die`)
    (`/Game/Blueprints/BP_Mario.On Jump on Enemy` _asbp_mario)))

(event `onDieByHit`
  (bind _sm_koopa (`self.SM_Koopa`))
  (bind _sm_koopa_2 (`self.SM_Koopa`))
  ;[1 1 1] Die
  (set `self.isDead` true)
  (set `self.isRotating` 0)
  (bind (_new_location _new_rotation) (`self.DieByHitAnimationUp` _sm_koopa))
  (`KismetSystemLibrary.MoveComponentTo` _sm_koopa _new_location _new_rotation false false 0.5)
  (bind (_new_location_2 _new_rotation_2) (`self.DieByHitAnimationDown` _sm_koopa_2))
  (`KismetSystemLibrary.MoveComponentTo` _sm_koopa_2 _new_location_2 _new_rotation_2 false false 0.5)
  (`KismetSystemLibrary.Delay` 1.0)
  (`self.K2_DestroyActor`))

(event `self.Collider_Top_Shell.OnComponentBeginOverlap`
  (params (OverlappedComponent :type "PrimitiveComponent Object Reference") (OtherActor :type "Actor Object Reference") (OtherComp :type "PrimitiveComponent Object Reference") (OtherBodyIndex :type Integer) (bFromSweep :type Boolean) (SweepResult :type "HitResult Structure (by ref)"))
  ;[1 0.04144 0.06134] Kill Koopa
  (if (not (`self.isDead`))
    (bind _asbp_mario (cast `/Game/Blueprints/BP_Mario` OtherActor))
    (`self.On Die`)
    (`/Game/Blueprints/BP_Mario.On Jump on Enemy` _asbp_mario)))

(fn `DieByHitAnimationDown`
  (params (Mesh :type "StaticMeshComponent Object Reference"))
  (returns (`New Location` :type "Vector Structure") (`New Rotation` :type "Rotator Structure"))
  (bind (_relativelocation_x _relativelocation_y _relativelocation_z) (`KismetMathLibrary.BreakVector` (`SceneComponent.RelativeLocation` Mesh)))
  (return (`KismetMathLibrary.MakeVector` _relativelocation_x _relativelocation_y (+ _relativelocation_z -320.0)) (`SceneComponent.RelativeRotation` Mesh)))

(fn `DieByHitAnimationUp`
  (params (Mesh :type "StaticMeshComponent Object Reference"))
  (returns (`New Location` :type "Vector Structure") (`New Rotation` :type "Rotator Structure"))
  (bind (_relativerotation_roll _relativerotation_pitch _relativerotation_yaw) (`KismetMathLibrary.BreakRotator` (`SceneComponent.RelativeRotation` Mesh)))
  (bind (_relativelocation_x _relativelocation_y _relativelocation_z) (`KismetMathLibrary.BreakVector` (`SceneComponent.RelativeLocation` Mesh)))
  (return (`KismetMathLibrary.MakeVector` _relativelocation_x _relativelocation_y (+ _relativelocation_z 160.0)) (`KismetMathLibrary.MakeRotator` (+ _relativerotation_roll -180.0) _relativerotation_pitch _relativerotation_yaw)))

(fn `Flip`
  (params (Degree :type "Float (double-precision)") (Mesh :type "StaticMeshComponent Object Reference"))
  (returns (`New Rotation` :type "Rotator Structure"))
  (bind (_relativerotation_roll _relativerotation_pitch _relativerotation_yaw) (`KismetMathLibrary.BreakRotator` (`SceneComponent.RelativeRotation` Mesh)))
  (return (`KismetMathLibrary.MakeRotator` _relativerotation_roll _relativerotation_pitch (+ Degree _relativerotation_yaw))))

(fn `GoBackward`
  (params (Mesh :type "StaticMeshComponent Object Reference"))
  (returns (`New Position` :type "Vector Structure") (`New Rotation` :type "Rotator Structure"))
  (bind (_relativelocation_x _relativelocation_y _relativelocation_z) (`KismetMathLibrary.BreakVector` (`SceneComponent.RelativeLocation` Mesh)))
  (return (`KismetMathLibrary.MakeVector` _relativelocation_x (- (`self.MoveDistance`) _relativelocation_y) _relativelocation_z) (`SceneComponent.RelativeRotation` Mesh)))

(fn `GoForward`
  (params (Mesh :type "StaticMeshComponent Object Reference"))
  (returns (`New Position` :type "Vector Structure") (`New Rotation` :type "Rotator Structure"))
  (bind (_relativelocation_x _relativelocation_y _relativelocation_z) (`KismetMathLibrary.BreakVector` (`SceneComponent.RelativeLocation` Mesh)))
  (bind (_relativerotation_roll _relativerotation_pitch _relativerotation_yaw) (`KismetMathLibrary.BreakRotator` (`SceneComponent.RelativeRotation` Mesh)))
  (return (`KismetMathLibrary.MakeVector` _relativelocation_x (+ (* (`self.DistanceY`) (`self.Direction`)) _relativelocation_y) (- _relativelocation_z (* (`self.DistanceZ`) (`self.isFalling`)))) (`KismetMathLibrary.MakeRotator` _relativerotation_roll _relativerotation_pitch (+ _relativerotation_yaw (* (`self.isRotating`) 60.0)))))

(fn `UserConstructionScript`)